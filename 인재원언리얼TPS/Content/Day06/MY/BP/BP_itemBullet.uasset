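; BP_itemBullet is a bullet pickup item that gives ammo to the player.
; When the player pawn overlaps it, it runs Work, then destroys itself after a short delay.
; Work sends AddBulletMessage with a fixed amount straight to the overlapping actor without casting; an older ThirdPersonCharacter cast calling AddBullet remains unconnected.
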(event `self.ReceiveActorBeginOverlap`
  (params (OtherActor :type "Actor Object Reference"))
  (if (== OtherActor (`GameplayStatics.GetPlayerPawn` 0))
    (`self.Work` OtherActor)
    (`KismetSystemLibrary.Delay` 0.2)
    (`self.K2_DestroyActor`)))

(fn `UserConstructionScript`)

(fn `Work`
  (params (otherActor :type "Actor Object Reference"))
  (message `/Game/Day06/MY/BP/BPI_Player.AddBullet` otherActor 100))