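; BP_TargetItem00 is a collectible target item that takes a random look and disappears when the player touches it.
; On BeginPlay it picks a random index from three, stores it in CheckNum and applies that entry of the Materials array to its Root mesh.
; On actor overlap it destroys itself if the other actor casts to ThirdPersonCharacter.
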(event `self.ReceiveBeginPlay`
  (bind _output_get (set `self.CheckNum` (`KismetMathLibrary.RandomInteger` 3)))
  (`PrimitiveComponent.SetMaterial` (`self.Root`) 0 (`|GetArrayItem` (`self.materials`) _output_get)))

(event `self.ReceiveTick`
  (params (DeltaSeconds :type "Float (single-precision)")))

(event `self.ReceiveActorBeginOverlap`
  (params (OtherActor :type "Actor Object Reference"))
  (cast `/Game/ThirdPersonBP/Blueprints/ThirdPersonCharacter` OtherActor)
  (`self.K2_DestroyActor`))

(fn `UserConstructionScript`)