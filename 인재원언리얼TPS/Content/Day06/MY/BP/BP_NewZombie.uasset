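; BP_NewZombie is an AI zombie enemy whose stats load from a Monster DataTable row during construction into a CharStat component.
; The component receives incoming damage and drives the health text, walk speed and death, which disables collision and destroys the actor after a delay.
; ANAttackTarget damages the Blackboard's PlayerCharacter if within range.
; RadialDamage pushes the zombie away from the hit origin with an impulse.
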(event `self.ReceiveBeginPlay`
  (set `self.SpawnLocation` (`self.K2_GetActorLocation`))
  (bind _aswb_char_status (cast `/Game/Day06/MY/UI/WB_CharStatus` (`WidgetComponent.GetUserWidgetObject` (`self.Widget`))))
  (set `/Game/Day06/MY/UI/WB_CharStatus.CharStatCompo` (`self.BP_CharStatComponent`) _aswb_char_status))

(event `self.ReceiveTick`
  (params (DeltaSeconds :type "Float (single-precision)")))

(event `self.ReceiveAnyDamage`
  (params (Damage :type "Float (single-precision)") (DamageType :type "DamageType Object Reference") (InstigatedBy :type "Controller Object Reference") (DamageCauser :type "Actor Object Reference"))
  (bind _returnvalue (`Controller.K2_GetPawn` InstigatedBy))
  (`/Engine/EditorBlueprintResources/StandardMacros.IsValid` _returnvalue
    (:`Is Valid`
      (`/Game/Day06/MY/BP/BP_CharStatComponent.TakeDamage` (`self.BP_CharStatComponent`) Damage _returnvalue))))

(event `self.BP_CharStatComponent.OnChangeHealth`
  (params (NewHealth :type "Float (single-precision)"))
  (`TextRenderComponent.K2_SetText` (`self.TextRender`) (`KismetTextLibrary.Conv_DoubleToText` NewHealth "HalfToEven")))

(event `self.BP_CharStatComponent.OnChangeSpeed`
  (params (NewSpeed :type "Float (single-precision)"))
  (set `CharacterMovementComponent.MaxWalkSpeed` NewSpeed (`self.CharacterMovement`)))

(event `self.BP_CharStatComponent.OnDeath`
  (set `self.Status` (struct :`TagName` "Status.Death"))
  (`PrimitiveComponent.SetCollisionEnabled` (`self.CapsuleComponent`) "NoCollision")
  (`PrimitiveComponent.SetCollisionEnabled` (`self.Mesh`) "NoCollision")
  (set `CharacterMovementComponent.MaxWalkSpeed` 0.0 (`self.CharacterMovement`))
  (`KismetSystemLibrary.Delay` 3.0)
  (`self.K2_DestroyActor`))

(event `/Game/Day06/MY/BP/BPI_AnimNotify.AN_AttackTarget`
  (params (Distance :type "Float (single-precision)"))
  (bind _returnvalue (`AIBlueprintHelperLibrary.GetAIController` self))
  (bind _returnvalue_2 (`AIBlueprintHelperLibrary.GetBlackboard` _returnvalue))
  (bind _returnvalue_3 (`BlackboardComponent.GetValueAsObject` _returnvalue_2 "PlayerCharacter"))
  (`/Engine/EditorBlueprintResources/StandardMacros.IsValid` _returnvalue
    (:`Is Valid`
      (`/Engine/EditorBlueprintResources/StandardMacros.IsValid` _returnvalue_2
        (:`Is Valid`
          (`/Engine/EditorBlueprintResources/StandardMacros.IsValid` _returnvalue_3
            (:`Is Valid`
              (bind _ascharacter (cast `Character` _returnvalue_3))
              (if (<= (`self.GetDistanceTo` _ascharacter) Distance)
                (`GameplayStatics.ApplyDamage` _ascharacter (`/Game/Day06/MY/BP/BP_CharStatComponent.Attack` (`self.BP_CharStatComponent`)) (`self.GetController`) self)))))))))

(event `/Game/Day06/MY/BP/BPI_Monster.SetStatus`
  (params (NewStatus :type "GameplayTag Structure"))
  (set `self.Status` NewStatus))

(event `self.ReceiveRadialDamage`
  (params (DamageReceived :type "Float (single-precision)") (DamageType :type "DamageType Object Reference") (Origin :type "Vector Structure") (HitInfo :type "HitResult Structure (by ref)") (InstigatedBy :type "Controller Object Reference") (DamageCauser :type "Actor Object Reference"))
  (`MovementComponent.StopMovementImmediately` (`self.CharacterMovement`))
  (`CharacterMovementComponent.AddImpulse` (`self.CharacterMovement`) (* (`KismetMathLibrary.Normal` (- (`self.K2_GetActorLocation`) Origin)) 1000000.0) false))

(fn `GetMonsterTableID`
  (returns (NormalMonsterID :type Integer) (HardMonsterID :type Integer))
  (return (`self.NormalMonsterTableID`) (`self.HardMonsterTableID`)))

(fn `GetStatus`
  (returns (Status :type "GameplayTag Structure"))
  (return (`self.Status`)))

(fn `TestFunction`)

(fn `UserConstructionScript`
  (bind _returnvalue (`|GetDataTableRow` "/Game/Day06/MY/BP/Excel/Monster.Monster" (`KismetStringLibrary.Conv_StringToName` (`KismetStringLibrary.Conv_IntToString` (`self.NormalMonsterTableID`))))
    (:`then`
      (bind (_level _name _speed _attack _health _defence) (break `/Game/Day06/MY/BP/MonsterStruct` _returnvalue))
      (set `/Game/Day06/MY/BP/BP_CharStatComponent.InitialStat` (make `/Game/Day06/MY/BP/F_InitialCharStat` _name _level _health _attack _defence _speed) (`self.BP_CharStatComponent`)))))