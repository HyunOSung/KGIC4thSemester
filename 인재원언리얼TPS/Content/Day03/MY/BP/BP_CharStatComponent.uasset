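; Character stat component that holds health, speed and attack, seeding health and attack from InitialStat at BeginPlay.
; AddHealth updates Health and HPPercent without clamping, and each stat setter fires its OnChange dispatcher for listeners.
; SetSpeedTempo applies a timed speed buff, flagged by OnBuffSPD, and a named timer calls ResetSpeed to restore the initial MoveSpeed.
; SetAttackTempo is an empty stub.
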(event `self.ReceiveBeginPlay`
  (bind (_initialstat_name _initialstat_health _initialstat_attack) (break `/Game/Day03/MY/BP/F_InitailCharStat` (`self.InitialStat`)))
  (`self.AddHealth` _initialstat_health)
  (`self.SetAttack` _initialstat_attack))

(fn `AddHealth`
  (params (value :type "Float (double-precision)"))
  (bind (_initialstat_name _initialstat_health) (break `/Game/Day03/MY/BP/F_InitailCharStat` (`self.InitialStat`)))
  (bind _output_get (set `self.Health` (+ value (`self.Health`))))
  (set `self.HPPercent` (/ _output_get _initialstat_health))
  (`self.OnChangeHealth` _output_get))

(fn `ResetSpeed`
  (bind (_initialstat_name _initialstat_health _initialstat_attack _initialstat_deffence _initialstat_movespeed) (break `/Game/Day03/MY/BP/F_InitailCharStat` (`self.InitialStat`)))
  (set `self.OnBuff_SPD` false)
  (`self.SetSpeed` _initialstat_movespeed))

(fn `SetAttack`
  (params (NewAttack :type "Float (double-precision)"))
  (bind _output_get (set `self.Attack` NewAttack))
  (`self.OnChangeAttack` _output_get))

(fn `SetAttackTempo`
  (params (NewAttack :type "Float (double-precision)") (Duration :type "Float (double-precision)")))

(fn `SetSpeed`
  (params (NewSpeed :type "Float (double-precision)"))
  (bind _output_get (set `self.Speed` NewSpeed))
  (`self.OnChangeSpeed` _output_get))

(fn `SetSpeedTempo`
  (params (NewSpeed :type "Float (double-precision)") (Duration :type "Float (double-precision)"))
  (bind _output_get (set `self.OnBuff_SPD` true))
  (`KismetSystemLibrary.PrintString` (`KismetStringLibrary.Conv_BoolToString` _output_get))
  (`self.SetSpeed` NewSpeed)
  (`KismetSystemLibrary.K2_SetTimer` self "ResetSpeed" Duration))