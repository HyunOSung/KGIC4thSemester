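; Spawner actor that scatters BP_Coin actors at random surface points inside its Box, though its IsValidClaas check returns false, gating off all BeginPlay logic.
; BeginPlay is written to call Spawn Total times, each retrying downward WorldStatic line traces until one hits, with debug drawing.
; With UseRespawn, destroyed coins increment a counter and unpause a looping timer, which respawns one per interval and pauses at zero.
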(event `self.ReceiveBeginPlay`
  (bind _newparam (`self.IsValidClaas`))
  (if _newparam
    (`|ExecutionSequence`
      (:`then_0`
        (if (`self.UseRespawn`)
          (bind _returnvalue (`KismetSystemLibrary.K2_SetTimerDelegate` (delegate `EventRespawn`) (`self.RespawnInterval`) true))
          (bind _output_get (set `self.RespawnTimerHandle` _returnvalue))
          (`KismetSystemLibrary.K2_PauseTimerHandle` _output_get)))
      (:`then_1`
        (for _ (range (`self.total`))
          (bind _newparam_2 (`self.Spawn` :!label _label))
          (if (`self.UseRespawn`)
            (add `self.OnDestroyed` _newparam_2 (delegate `DestroyEvent`))))))))

(event `EventRespawn`
  (bind _destroyedactor (`self.DestroyedActor`))
  (`/Engine/EditorBlueprintResources/StandardMacros.CompareInt` _destroyedactor
    (:`>`
      (`/Engine/EditorBlueprintResources/StandardMacros.DecrementInt` _destroyedactor
        (:`  `
          (goto _label))))
    (:`==`
      (`KismetSystemLibrary.K2_PauseTimerHandle` (`self.RespawnTimerHandle`)))))

(event `Key|One`
  (params (Key :type "Key Structure"))
  (:`Pressed`
    (`KismetSystemLibrary.PrintString` "Hello")))

(event `DestroyEvent` :!signature `self.OnDestroyed`
  (params (DestroyedActor :type "Actor Object Reference"))
  (`/Engine/EditorBlueprintResources/StandardMacros.IncrementInt` (`self.DestroyedActor`)
    (:`  `
      (`KismetSystemLibrary.K2_UnPauseTimerHandle` (`self.RespawnTimerHandle`)))))

(fn `IsValidClaas`
  (returns (NewParam :type Boolean))
  (return false))

(fn `Spawn`
  (returns (NewParam :type "Actor Object Reference"))
  (bind _box (`self.Box`))
  (bind _returnvalue (`SceneComponent.K2_GetComponentLocation` _box))
  (bind _returnvalue_2 (`BoxComponent.GetScaledBoxExtent` _box))
  (bind _z (.z _returnvalue_2))
  (bind _z_2 (.z _returnvalue))
  (bind _x (.x (`KismetMathLibrary.RandomPointInBoundingBox` _returnvalue _returnvalue_2)))
  (bind _y (.y (`KismetMathLibrary.RandomPointInBoundingBox` _returnvalue _returnvalue_2)))
  (bind (_outhit _returnvalue_3) (`KismetSystemLibrary.LineTraceSingleForObjects` :`Start` (`KismetMathLibrary.MakeVector` _x _y (+ _z_2 _z)) :`End` (`KismetMathLibrary.MakeVector` _x _y (- _z_2 _z)) :`ObjectTypes` (`|MakeArray` "ObjectTypeQuery1" :!type "EObjectTypeQuery Enum") :`DrawDebugType` "ForDuration" :`DrawTime` 1.0 :!label _label))
  (if _returnvalue_3
    (bind (_bblockinghit _binitialoverlap _time _distance _location) (`GameplayStatics.BreakHitResult` _outhit))
    (`KismetSystemLibrary.DrawDebugSphere` _location 100.0 12 (struct :`R` 1.0 :`G` 1.0 :`B` 1.0 :`A` 1.0) 1.0)
    (bind _returnvalue_4 (`|SpawnActorFromClass` "/Game/Day06/MY/BP/BP_Coin.BP_Coin_C" (`KismetMathLibrary.MakeTransform` _location) "Undefined" "OverrideRootScale" null null))
    (return _returnvalue_4)
    (else
      (goto _label))))

(fn `UserConstructionScript`)