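; Zombie enemy character that patrols around its spawn point, chases pawns it sees, attacks them and is destroyed shortly after death.
; Tick runs a gameplay-tag state machine with AI MoveTo, while PawnSensing sets the target, which is dropped after a timeout.
; Construction loads stats from a Monster data table into a stat component that handles damage and drives health text, walk speed and death.
; ANAttackTarget applies attack damage to the target.
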(event `self.ReceiveBeginPlay`
  (set `self.SpawnLocation` (`self.K2_GetActorLocation`))
  (bind _aswb_char_status (cast `/Game/Day06/MY/UI/WB_CharStatus` (`WidgetComponent.GetUserWidgetObject` (`self.Widget`))))
  (set `/Game/Day06/MY/UI/WB_CharStatus.CharStatCompo` (`self.BP_CharStatComponent`) _aswb_char_status))

(event `self.ReceiveTick`
  (params (DeltaSeconds :type "Float (single-precision)"))
  (`|ExecutionSequence`
    (:`then_0`
      (`/Engine/EditorBlueprintResources/StandardMacros.IsValid` (`self.TargetPawn`)
        (:`Is Valid`
          (if (> (- (`GameplayStatics.GetTimeSeconds`) (`self.TargetLastTime`)) (`self.TargetLostTime`))
            (set `self.TargetPawn` null)
            (`Controller.StopMovement` (`AIBlueprintHelperLibrary.GetAIController` self))
            (set `self.Status` (struct :`TagName` "Status.Idle"))))))
    (:`then_1`
      (if (`|EnumEquality` (`AIController.GetMoveStatus` (`AIBlueprintHelperLibrary.GetAIController` self)) "Idle")
        (`|SwitchGameplayTag` (`self.Status`)
          (:`Status.Idle`
            (`KismetSystemLibrary.Delay` 1.0)
            (set `self.Status` (struct :`TagName` "Status.Patrol")))
          (:`Status.Patrol`
            (`|AIMoveTo` self (`NavigationSystemV1.K2_GetRandomReachablePointInRadius` (`self.SpawnLocation`) 500.0 null null) null
              (:`OnSuccess`
                _)
              (:`OnFail`
                _))
            (set `self.Status` (struct :`TagName` "Status.Idle")))
          (:`Status.Trace`
            (`|AIMoveTo` self (0.0 0.0 0.0) (`self.TargetPawn`)
              (:`OnSuccess`
                (set `self.Status` (struct :`TagName` "Status.Attack")))
              (:`OnFail`
                (set `self.Status` (struct :`TagName` "Status.Idle"))))))))))

(event `self.PawnSensing.OnSeePawn`
  (params (Pawn :type "Pawn Object Reference"))
  (`self.TargetPawn`
    (:`then`
      _)
    (:`else`
      (set `self.TargetPawn` Pawn)
      (set `self.Status` (struct :`TagName` "Status.Trace"))))
  (set `self.TargetLastTime` (`KismetSystemLibrary.GetGameTimeInSeconds`)))

(event `self.ReceiveAnyDamage`
  (params (Damage :type "Float (single-precision)") (DamageType :type "DamageType Object Reference") (InstigatedBy :type "Controller Object Reference") (DamageCauser :type "Actor Object Reference"))
  (bind _returnvalue (`Controller.K2_GetPawn` InstigatedBy))
  (`/Engine/EditorBlueprintResources/StandardMacros.IsValid` _returnvalue
    (:`Is Valid`
      (`/Game/Day06/MY/BP/BP_CharStatComponent.TakeDamage` (`self.BP_CharStatComponent`) Damage _returnvalue))))

(event `self.BP_CharStatComponent.OnChangeHealth`
  (params (NewHealth :type "Float (single-precision)"))
  (`TextRenderComponent.K2_SetText` (`self.TextRender`) (`KismetTextLibrary.Conv_DoubleToText` NewHealth "HalfToEven")))

(event `self.BP_CharStatComponent.OnChangeSpeed`
  (params (NewSpeed :type "Float (single-precision)"))
  (set `CharacterMovementComponent.MaxWalkSpeed` NewSpeed (`self.CharacterMovement`)))

(event `self.BP_CharStatComponent.OnDeath`
  (set `self.Status` (struct :`TagName` "Status.Death"))
  (`PrimitiveComponent.SetCollisionEnabled` (`self.CapsuleComponent`) "NoCollision")
  (`PrimitiveComponent.SetCollisionEnabled` (`self.Mesh`) "NoCollision")
  (set `CharacterMovementComponent.MaxWalkSpeed` 0.0 (`self.CharacterMovement`))
  (`KismetSystemLibrary.Delay` 3.0)
  (`self.K2_DestroyActor`))

(event `/Game/Day06/MY/BP/BPI_AnimNotify.AN_AttackTarget`
  (`GameplayStatics.ApplyDamage` (`self.TargetPawn`) (`/Game/Day06/MY/BP/BP_CharStatComponent.Attack` (`self.BP_CharStatComponent`)) (`self.GetController`) self))

(event `/Game/Day06/MY/BP/BPI_Monster.SetStatus`
  (params (NewStatus :type "GameplayTag Structure"))
  (set `self.Status` NewStatus))

(fn `GetMonsterTableID`
  (returns (NormalMonsterID :type Integer) (HardMonsterID :type Integer))
  (return 0 0))

(fn `GetStatus`
  (returns (Status :type "GameplayTag Structure"))
  (return (`self.Status`)))

(fn `TestFunction`)

(fn `UserConstructionScript`
  (bind _returnvalue (`|GetDataTableRow` "/Game/Day06/MY/BP/Excel/Monster.Monster" (`KismetStringLibrary.Conv_StringToName` (`KismetStringLibrary.Conv_IntToString` (`self.MonsterTableID`))))
    (:`then`
      (bind (_level _name _speed _attack _health _defence) (break `/Game/Day06/MY/BP/MonsterStruct` _returnvalue))
      (set `/Game/Day06/MY/BP/BP_CharStatComponent.InitialStat` (make `/Game/Day06/MY/BP/F_InitialCharStat` _name _level _health _attack _defence _speed) (`self.BP_CharStatComponent`)))))