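; Grenade pickup item that gives grenades to the player who walks over it.
; On overlap with the player pawn, Work sends AddGrenadeMessage with a fixed amount to that actor, then the item destroys itself after a short delay.
; The effect goes through an interface message, so the live path needs no cast; an unused ThirdPersonCharacter cast calling AddBullet remains disconnected in Work.
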(event `self.ReceiveActorBeginOverlap`
  (params (OtherActor :type "Actor Object Reference"))
  ;[1 1 1] 8주차 이전에 만든 아이템 블루프린트 활용해서 수류탄 아이템을 만듬
  (if (== OtherActor (`GameplayStatics.GetPlayerPawn` 0))
    (`self.Work` OtherActor)
    (`KismetSystemLibrary.Delay` 0.2)
    (`self.K2_DestroyActor`)))

(fn `UserConstructionScript`)

(fn `Work`
  (params (otherActor :type "Actor Object Reference"))
  ;[1 1 1] 8주차 인터페이스를 통해 아이템 효과 플레이어에 전달
  (message `/Game/Day06/MY/BP/BPI_Player.AddGrenade` otherActor 10))