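; BP_Lift is a lift platform that rises and lowers in response to a lever.
; At BeginPlay it casts its child actor to BP_Lever, binds to that lever's switch-change event and records the Plane's starting world location.
; Switching on plays a timeline whose Height track offsets the Plane's Z from that location; switching off reverses the timeline.
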(event `self.ReceiveBeginPlay`
  (bind _asbp_lever (cast `/Game/Day06/MY/BP/BP_Lever` (`ChildActorComponent.ChildActor` (`self.ChildActor`))))
  (add `/Game/Day06/MY/BP/BP_Lever.OnChangeSwitch` _asbp_lever (delegate `커스텀이벤트_0`))
  (set `self.SpawnLocation` (`SceneComponent.K2_GetComponentLocation` (`self.Plane`))))

(event `커스텀이벤트_0`
  (params (Switch :type Boolean))
  (bind (_spawnlocation_x _spawnlocation_y _spawnlocation_z) (`KismetMathLibrary.BreakVector` (`self.SpawnLocation`)))
  (if Switch
    (bind (_direction _height) (`Timeline|타임라인_0` :`NewTime` (`GameplayStatics.GetTimeSeconds`) :!label _label)
      (:`Update`
        (`SceneComponent.K2_SetWorldLocation` (`self.Plane`) (`KismetMathLibrary.MakeVector` _spawnlocation_x _spawnlocation_y (+ _spawnlocation_z _height)) false false)))
    (else
      (goto _label :!via `Reverse`))))

(fn `UserConstructionScript`)