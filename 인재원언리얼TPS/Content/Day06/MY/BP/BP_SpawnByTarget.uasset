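; Spawner actor that places a random class from SpawnActorClass at each TargetPointClass actor attached to itself or its attach parent.
; BeginPlay validates the classes, collects point locations into SpawnLocationArray and spawns at each one.
; With UseRespawn, destroyed actors append their location to that same array and unpause a looping timer.
; The timer respawns from the array's front and pauses when empty; initial locations remain queued after the first spawn.
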(event `self.ReceiveBeginPlay`
  (bind _newparam (`self.IsValidClaas`))
  (if _newparam
    (`self.InitSpawnLocation`)
    (`|ExecutionSequence`
      (:`then_0`
        (if (`self.UseRespawn`)
          (bind _returnvalue (`KismetSystemLibrary.K2_SetTimerDelegate` (delegate `EventRespawn`) (`self.RespawnInterval`) true))
          (bind _output_get (set `self.RespawnTimerHandle` _returnvalue))
          (`KismetSystemLibrary.K2_PauseTimerHandle` _output_get)))
      (:`then_1`
        (for _array_element (`self.SpawnLocationArray`)
          (set `self.TempSpawnLocation` _array_element)
          (bind _newparam_2 (`self.Spawn` (`self.TempSpawnLocation`) :!label _label))
          (if (`self.UseRespawn`)
            (add `self.OnDestroyed` _newparam_2 (delegate `DestroyEvent`))))))))

(event `EventRespawn`
  (bind _spawnlocationarray (`self.SpawnLocationArray`))
  (`/Engine/EditorBlueprintResources/StandardMacros.CompareInt` (`KismetArrayLibrary.Array_Length` _spawnlocationarray)
    (:`>`
      (set `self.TempSpawnLocation` (`|GetArrayItem` _spawnlocationarray))
      (`KismetArrayLibrary.Array_Remove` _spawnlocationarray)
      (goto _label))
    (:`==`
      (`KismetSystemLibrary.K2_PauseTimerHandle` (`self.RespawnTimerHandle`)))))

(event `Key|One`
  (params (Key :type "Key Structure"))
  (:`Pressed`
    (`KismetSystemLibrary.PrintString` "Hello")))

(event `DestroyEvent`
  (params (DestroyedActor :type "Actor Object Reference"))
  (`KismetArrayLibrary.Array_Add` (`self.SpawnLocationArray`) (`self.K2_GetActorLocation` DestroyedActor))
  (`KismetSystemLibrary.K2_UnPauseTimerHandle` (`self.RespawnTimerHandle`)))

(fn `AttachSpawnTargetPoint`
  (bind _returnvalue (`|SpawnActorFromClass` (`self.TargetPointClass`) (`KismetMathLibrary.MakeTransform` (0.0 0.0 0.0)) "Undefined" "OverrideRootScale" null null))
  (`self.K2_AttachToActor` _returnvalue self "None" "KeepRelative" "KeepRelative" "KeepRelative" true))

(fn `InitSpawnLocation`
  (locals (LocalTempActor :type "Actor Object Reference"))
  (bind _returnvalue (`self.GetAttachParentActor`))
  (`|ExecutionSequence`
    (:`then_0`
      (set `local.LocalTempActor` self))
    (:`then_1`
      (`/Engine/EditorBlueprintResources/StandardMacros.IsValid` _returnvalue
        (:`Is Valid`
          (set `local.LocalTempActor` _returnvalue)))))
  (for _array_element (`self.GetAttachedActors` (`local.LocalTempActor`) true)
    (if (== (`GameplayStatics.GetObjectClass` _array_element) (`self.TargetPointClass`))
      (`KismetArrayLibrary.Array_Add` (`self.SpawnLocationArray`) (`self.K2_GetActorLocation` _array_element)))))

(fn `IsValidClaas`
  (returns (NewParam :type Boolean))
  (bind _spawnactorclass (`self.SpawnActorClass`))
  (if (`KismetSystemLibrary.IsValidClass` (`self.TargetPointClass`))
    (if (> (`KismetArrayLibrary.Array_Length` _spawnactorclass) 0)
      (for _array_element _spawnactorclass
        (if (not (`KismetSystemLibrary.IsValidClass` _array_element))
          (return false)))
      (return true)
      (else
        _)))
  (return false))

(fn `Spawn`
  (params (Location :type "Vector Structure"))
  (returns (NewParam :type "Actor Object Reference"))
  (bind _returnvalue (`|SpawnActorFromClass` (`|GetArrayItem` (`self.SpawnActorClass`) (`KismetMathLibrary.RandomInteger` (`KismetArrayLibrary.Array_Length` (`self.SpawnActorClass`)))) (`KismetMathLibrary.MakeTransform` Location) "Undefined" "OverrideRootScale" null null))
  (return _returnvalue))

(fn `UserConstructionScript`)