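; BP_CharStatComponent is a character stat component holding health, speed and attack, seeding health and attack from InitialStat on BeginPlay.
; Setters broadcast speed and attack changes; AddHealth updates HPPercent before clamping and broadcasts only when clamped, using a hardcoded 100 upper threshold.
; Timed buffs replace speed or add to attack, set a flag, then use named-function timers to restore InitialStat values and broadcast the buff's end.
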(event `self.ReceiveBeginPlay`
  (bind (_initialstat_name _initialstat_health _initialstat_attack) (break `/Game/Day06/MY/BP/F_InitailCharStat` (`self.InitialStat`)))
  (`self.AddHealth` _initialstat_health)
  (`self.SetAttack` _initialstat_attack)
  (`KismetSystemLibrary.PrintString` (`KismetStringLibrary.Conv_DoubleToString` (`self.Attack`))))

(fn `AddHealth`
  (params (value :type "Float (double-precision)"))
  (bind (_initialstat_name _initialstat_health) (break `/Game/Day06/MY/BP/F_InitailCharStat` (`self.InitialStat`)))
  (bind (_initialstat_name_2 _initialstat_health_2) (break `/Game/Day06/MY/BP/F_InitailCharStat` (`self.InitialStat`)))
  (bind _output_get (set `self.Health` (+ value (`self.Health`))))
  (set `self.HPPercent` (/ _output_get _initialstat_health))
  (if (< (`self.Health`) 0.0)
    (set `self.Health` 0.0)
    (`self.OnChangeHealth` _output_get :!label _label)
    (elif (> (`self.Health`) 100.0)
      (set `self.Health` _initialstat_health_2)
      (goto _label))))

(fn `ResetAttack`
  (bind (_initialstat_name _initialstat_health _initialstat_attack) (break `/Game/Day06/MY/BP/F_InitailCharStat` (`self.InitialStat`)))
  (set `self.OnBuff_ATK` false)
  (`self.SetAttack` _initialstat_attack)
  (`self.ATKBuffEnd`))

(fn `ResetSpeed`
  (bind (_initialstat_name _initialstat_health _initialstat_attack _initialstat_deffence _initialstat_movespeed) (break `/Game/Day06/MY/BP/F_InitailCharStat` (`self.InitialStat`)))
  (set `self.OnBuff_SPD` false)
  (`self.SetSpeed` _initialstat_movespeed)
  (`self.SPDBuffEnd`))

(fn `SetAttack`
  (params (NewAttack :type "Float (double-precision)"))
  (bind _output_get (set `self.Attack` NewAttack))
  (`self.OnChangeAttack` _output_get))

(fn `SetAttackTempo`
  (params (NewAttack :type "Float (double-precision)") (Duration :type "Float (double-precision)"))
  (set `self.OnBuff_ATK` true)
  (`self.SetAttack` (+ NewAttack (`self.Attack`)))
  (`KismetSystemLibrary.K2_SetTimer` self "ResetAttack" Duration))

(fn `SetSpeed`
  (params (NewSpeed :type "Float (double-precision)"))
  (bind _output_get (set `self.Speed` NewSpeed))
  (`self.OnChangeSpeed` _output_get))

(fn `SetSpeedTempo`
  (params (NewSpeed :type "Float (double-precision)") (Duration :type "Float (double-precision)"))
  (bind _output_get (set `self.OnBuff_SPD` true))
  (`KismetSystemLibrary.PrintString` (`KismetStringLibrary.Conv_BoolToString` _output_get))
  (`self.SetSpeed` NewSpeed)
  (`KismetSystemLibrary.K2_SetTimer` self "ResetSpeed" Duration))