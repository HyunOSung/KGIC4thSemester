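; BP_Enemy is an enemy that wanders at random, deals contact damage and can take damage itself.
; From BeginPlay it loops AIMoveTo toward random reachable points nearby, pausing briefly after each success or failure.
; Hits apply damage to the other actor, throttled by a time-based cooldown.
; Incoming damage lowers health in its character stat component, which is handed to its HP_New widget at startup.
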(event `self.ReceiveActorBeginOverlap`
  (params (OtherActor :type "Actor Object Reference")))

(event `self.ReceiveHit`
  (params (MyComp :type "PrimitiveComponent Object Reference") (Other :type "Actor Object Reference") (OtherComp :type "PrimitiveComponent Object Reference") (bSelfMoved :type Boolean) (HitLocation :type "Vector Structure") (HitNormal :type "Vector Structure") (NormalImpulse :type "Vector Structure") (Hit :type "HitResult Structure (by ref)"))
  (bind _returnvalue (`GameplayStatics.GetTimeSeconds`))
  (if (> (`KismetMathLibrary.Abs` (- (`self.LastDamageTime`) _returnvalue)) (`self.InputDamageDelay`))
    (`GameplayStatics.ApplyDamage` Other 10.0 null self)
    (set `self.LastDamageTime` _returnvalue)))

(event `self.ReceiveTick`
  (params (DeltaSeconds :type "Float (single-precision)")))

(event `self.ReceiveAnyDamage`
  (params (Damage :type "Float (single-precision)") (DamageType :type "DamageType Object Reference") (InstigatedBy :type "Controller Object Reference") (DamageCauser :type "Actor Object Reference"))
  (`/Game/Day06/MY/BP/BP_CharStatComponent.AddHealth` (`self.BP_CharStatComponent`) (* Damage -1.0)))

(event `self.ReceiveBeginPlay`
  (bind (_randomlocation _returnvalue) (`NavigationSystemV1.K2_GetRandomReachablePointInRadius` (`self.K2_GetActorLocation`) 500.0 null null))
  (bind _ashp_new (cast `/Game/Day06/MY/BP/HP_New` (`WidgetComponent.GetUserWidgetObject` (`self.Widget`))))
  (set `/Game/Day06/MY/BP/HP_New.CharStat` (`self.BP_CharStatComponent`) _ashp_new)
  (`|AIMoveTo` self _randomlocation null 5.0 _returnvalue :!label _label
    (:`OnSuccess`
      _)
    (:`OnFail`
      _))
  (`KismetSystemLibrary.Delay` 1.0)
  (goto _label))

(event `self.BP_CharStatComponent.OnChangeHealth`
  (params (NewHealth :type "Float (single-precision)")))

(fn `UserConstructionScript`)