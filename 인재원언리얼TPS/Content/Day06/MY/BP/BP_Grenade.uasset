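; Grenade projectile actor that explodes on a fixed timer after spawning.
; BeginPlay waits out the fuse, applies radial damage credited to the instigator, draws a debug sphere of the blast radius, plays sound and explosion particles, then destroys itself shortly after.
; SetSpeed sets both initial and max speed on its ProjectileMovement component.
; Overlap, Tick and Hit events are empty, so impacts do not trigger detonation.
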(event `self.ReceiveBeginPlay`
  (bind _returnvalue (`self.K2_GetActorLocation`))
  (`KismetSystemLibrary.Delay` 3.0)
  (`GameplayStatics.ApplyRadialDamage` :`BaseDamage` 100.0 :`Origin` _returnvalue :`DamageRadius` 500.0 :`DamageCauser` self :`InstigatedByController` (`self.GetInstigatorController`))
  (`KismetSystemLibrary.DrawDebugSphere` _returnvalue 500.0 12 (struct :`R` 1.0 :`G` 1.0 :`B` 1.0 :`A` 1.0) 1.0)
  (`GameplayStatics.PlaySoundAtLocation` "/Game/Day06/MY/Sound/GrenadeCue.GrenadeCue" _returnvalue (struct) 1.0 1.0 0.0 null null null)
  (`GameplayStatics.SpawnEmitterAtLocation` "/Game/Lecture/Effects/P_Explosion_Bomb.P_Explosion_Bomb" _returnvalue)
  (`KismetSystemLibrary.Delay` 0.2)
  (`self.K2_DestroyActor`))

(event `self.ReceiveHit`
  (params (MyComp :type "PrimitiveComponent Object Reference") (Other :type "Actor Object Reference") (OtherComp :type "PrimitiveComponent Object Reference") (bSelfMoved :type Boolean) (HitLocation :type "Vector Structure") (HitNormal :type "Vector Structure") (NormalImpulse :type "Vector Structure") (Hit :type "HitResult Structure (by ref)")))

(fn `SetSpeed`
  (params (`New Speed` :type "Float (double-precision)"))
  (bind _projectilemovement (`self.ProjectileMovement`))
  (set `ProjectileMovementComponent.InitialSpeed` `New Speed` _projectilemovement)
  (set `ProjectileMovementComponent.MaxSpeed` `New Speed` _projectilemovement))

(fn `UserConstructionScript`)