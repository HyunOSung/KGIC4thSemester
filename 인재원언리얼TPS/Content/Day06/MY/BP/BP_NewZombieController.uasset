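; AI controller for zombies that runs a data-driven behavior tree and feeds its blackboard.
; On possess, it picks the normal or hard monster ID by game level, then async-loads that Monster table row's behavior tree.
; It binds the pawn's stat component to keep HealthRate updated.
; Sight perception of Player-tagged actors sets SeePlayer and PlayerCharacter, clearing them after a short forget timer once sight is lost.
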(event `self.ReceivePossess`
  (params (PossessedPawn :type "Pawn Object Reference"))
  (bind _returnvalue (`self.GetComponentByClass` PossessedPawn "/Game/Day06/MY/BP/BP_CharStatComponent.BP_CharStatComponent_C"))
  (bind (_normalmonsterid _hardmonsterid) (message `/Game/Day06/MY/BP/BPI_Monster.GetMonsterTableID` PossessedPawn))
  (bind _asmy_game_mode (cast `/Game/Day06/MY/BP/MyGameMode` (`GameplayStatics.GetGameMode`)))
  (bind _returnvalue_2 (`|GetDataTableRow` "/Game/Day06/MY/BP/Excel/Monster.Monster" (`KismetStringLibrary.Conv_StringToName` (`KismetStringLibrary.Conv_IntToString` (`KismetMathLibrary.SelectInt` _normalmonsterid _hardmonsterid (`|EnumEquality` (`/Game/Day06/MY/BP/MyGameMode.GameLevel` _asmy_game_mode) "NewEnumerator0")))))
    (:`then`
      (bind _object (`|LoadAsset` (`.BehaiviorTreeAssetPath_18_1B69B5C045622190AAD7699BB401D7BF` (break `/Game/Day06/MY/BP/MonsterStruct` _returnvalue_2)))
        (:`Completed`
          (bind _asbehavior_tree (cast `BehaviorTree` _object))
          (`self.RunBehaviorTree` _asbehavior_tree)
          (`/Engine/EditorBlueprintResources/StandardMacros.IsValid` _returnvalue
            (:`Is Valid`
              (add `/Game/Day06/MY/BP/BP_CharStatComponent.OnChangeHealth` _returnvalue (delegate `EventUpdateBlackBoard`))
              ;[1 1 1] 빙의 순간 체력 비율 초기값 1 설정
              (`BlackboardComponent.SetValueAsFloat` (`self.Blackboard`) "HealthRate" (/ (`/Game/Day06/MY/BP/BP_CharStatComponent.Health` _returnvalue) (`.Health_5_6510B2CC429A8D17FCC2C5B7629840E5` (break `/Game/Day06/MY/BP/F_InitialCharStat` (`/Game/Day06/MY/BP/BP_CharStatComponent.InitialStat` _returnvalue))))))))))))

(event `EventUpdateBlackBoard`
  (params (NewHealth :type "Float (double-precision)"))
  ;[1 1 1] 변경될 때 체력 비율 설정
  (`BlackboardComponent.SetValueAsFloat` (`self.Blackboard`) "HealthRate" (/ NewHealth (`.Health_5_6510B2CC429A8D17FCC2C5B7629840E5` (break `/Game/Day06/MY/BP/F_InitialCharStat` (`/Game/Day06/MY/BP/BP_CharStatComponent.InitialStat` (`self.GetComponentByClass` (stale `self.ReceivePossess` PossessedPawn) "/Game/Day06/MY/BP/BP_CharStatComponent.BP_CharStatComponent_C")))))))

(event `self.AIPerception.OnTargetPerceptionUpdated`
  (params (Actor :type "Actor Object Reference") (Stimulus :type "AIStimulus Structure"))
  (`/Engine/EditorBlueprintResources/StandardMacros.IsValid` Actor
    (:`Is Valid`
      (if (`self.ActorHasTag` Actor "Player")
        (bind _returnvalue (`AIPerceptionSystem.GetSenseClassForStimulus` Stimulus))
        (if (== _returnvalue "/Script/AIModule.AISense_Sight")
          ;[1 1 1] Sensed true면 플레이어 보임, false면 플레이어 안보임
          (if (`.bSuccessfullySensed` (break `AIStimulus` Stimulus))
            (`KismetSystemLibrary.K2_ClearAndInvalidateTimerHandle` (`self.ForgetTimer`))
            (bind _blackboard (`self.Blackboard`)
              (:`then`
                (`BlackboardComponent.SetValueAsBool` _blackboard "SeePlayer" true)
                (`BlackboardComponent.SetValueAsObject` _blackboard "PlayerCharacter" Actor))
              (:`else`))
            (else
              (bind _returnvalue_2 (`KismetSystemLibrary.K2_SetTimerDelegate` (delegate `EventForget`) 1.5))
              (set `self.ForgetTimer` _returnvalue_2))))))))

(event `EventForget`
  ;[1 1 1] MaxAge값 3초를 이용해서 마지막으로 본 시간 이후 3초 뒤에 잊어버리기
  (bind _blackboard (`self.Blackboard`)
    (:`then`
      (`BlackboardComponent.SetValueAsBool` _blackboard "SeePlayer" false)
      (`BlackboardComponent.SetValueAsObject` _blackboard "PlayerCharacter" null))
    (:`else`)))

(fn `UserConstructionScript`)