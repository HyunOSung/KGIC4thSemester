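; BP_Lever is a switch lever actor that shows a text label while any actor overlaps it.
; Its Work event plays or reverses a timeline based on the Switch state, adding the timeline's angle to the lever mesh's pitch from its BeginPlay rotation.
; When the timeline finishes, Switch flips and the OnChangeSwitch dispatcher broadcasts the new state.
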(event `self.ReceiveBeginPlay`
  (set `self.SpawnRotation` (`SceneComponent.K2_GetComponentRotation` (`self.Lever`))))

(event `self.ReceiveActorBeginOverlap`
  (params (OtherActor :type "Actor Object Reference"))
  (`SceneComponent.SetVisibility` (`self.TextRender`) true false))

(event `self.ReceiveActorEndOverlap`
  (params (OtherActor :type "Actor Object Reference"))
  (`SceneComponent.SetVisibility` (`self.TextRender`) false false))

(event `/Game/Day06/MY/BP/BPI_Interaction.Work`
  (if (`self.Switch`)
    (bind (_direction _angle) (`Timeline|타임라인_0` :`NewTime` (`GameplayStatics.GetTimeSeconds`) :!via `Reverse` :!label _label)
      (:`Update`
        (`SceneComponent.K2_SetWorldRotation` (`self.Lever`) (`KismetMathLibrary.MakeRotator` (.roll (`self.SpawnRotation`)) (+ (.pitch (`self.SpawnRotation`)) _angle) (.yaw (`self.SpawnRotation`))) false false))
      (:`Finished`
        (bind _output_get (set `self.Switch` (not (`self.Switch`))))
        (`self.OnChangeSwitch` _output_get)))
    (else
      (goto _label))))

(fn `UserConstructionScript`)