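; BP_SlidingDoor is a sliding door that opens when an actor overlaps it and closes when the overlap ends.
; BeginPlay caches the static mesh's world location as the rest position.
; Overlap events play and reverse a timeline whose AddValue track offsets the mesh from that position along world X.
; Any overlapping actor triggers it, as there is no filtering.
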(event `self.ReceiveBeginPlay`
  (set `self.SpawnLocation` (`SceneComponent.K2_GetComponentLocation` (`self.StaticMesh`))))

(event `self.ReceiveActorBeginOverlap`
  (params (OtherActor :type "Actor Object Reference"))
  (bind (_direction _addvalue) (`Timeline|타임라인_0` :`NewTime` (`GameplayStatics.GetTimeSeconds`) :!label _label)
    (:`Update`
      (`SceneComponent.K2_SetWorldLocation` (`self.StaticMesh`) (`KismetMathLibrary.MakeVector` (+ (.x (`self.SpawnLocation`)) _addvalue) (.y (`self.SpawnLocation`)) (.z (`self.SpawnLocation`))) false false))))

(event `self.ReceiveActorEndOverlap`
  (params (OtherActor :type "Actor Object Reference"))
  (goto _label :!via `Reverse`))

(fn `UserConstructionScript`)